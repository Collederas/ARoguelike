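; Enemy AI controller for turn-based grid movement that chases the player once alerted.
; AI perception latches an Alerted flag when it senses a Player-tagged actor; nothing here clears it.
; On each turn tick, an alerted enemy retargets its RL path following component and moves one cell toward the player, while an unalerted one reports out of moves immediately.
; Successful moves report out of moves, and nearing the target fires a target-reached notification.
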(event `self.ReceivePossess`
  (params (PossessedPawn :type "Pawn Object Reference"))
  (bind _asbp_player_controller (cast `/Game/Blueprints/BP_PlayerController` (`GameplayStatics.GetPlayerController` 0)))
  (set `self.PlayerController` _asbp_player_controller))

(event `/Game/Blueprints/BP_TurnBasedObject.TickTurn`
  (bind _returnvalue (`self.K2_GetActorLocation` (`GameplayStatics.GetPlayerPawn` 0)))
  (if (`self.Alerted`)
    (bind _returnvalue_2 (`self.GetRLPathFollowingComponent`))
    (`RoguelikePathFollowingComponent.UpdateTargetLocation` _returnvalue_2 (`KismetMathLibrary.Conv_VectorToVector2D` _returnvalue))
    (set `self.LocationAtTurnStart` (`self.K2_GetActorLocation` (`self.K2_GetPawn`)))
    (`self.GridMoveTo` _returnvalue null 1)
    (else
      (`self.NotifyOutOfMoves` self))))

(event `self.OnMoveCompleted_Blueprint`
  (params (RequestID :type "AIRequestID Structure") (Result :type "EPathFollowingResult Enum" :default "Success"))
  (switch `EPathFollowingResult` Result
    (:`Success`
      (`self.NotifyOutOfMoves` self))))

(event `self.OnAboutToReachTarget`
  (`self.TargetReached`))

(event `self.AIPerception.OnTargetPerceptionUpdated`
  (params (Actor :type "Actor Object Reference") (Stimulus :type "AIStimulus Structure"))
  (if (and (`self.ActorHasTag` Actor "Player") Stimulus_bSuccessfullySensed)
    (set `self.Alerted` true)
    (else
      (`KismetSystemLibrary.PrintString` "Nonalerted"))))

(fn `GetAvailableMoves`
  (returns (NrOfMovesLeft :type Integer))
  (return 0))

(fn `GridMoveToLocation`
  (params (Location :type "Vector Structure") (NumberOfMoves :type Integer))
  (`self.GridMoveTo` Location null NumberOfMoves))

(fn `UserConstructionScript`)