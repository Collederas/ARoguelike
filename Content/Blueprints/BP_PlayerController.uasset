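; Player controller that turns movement input into directional move commands on the controlled BP_Player pawn.
; On BeginPlay it casts and caches the pawn, then each pressed Move action calls the matching forward, backward, left or right function on it.
; A TickTurn event re-enables the controller's input, suggesting turn-based movement; nothing in this Blueprint disables it.
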(event `self.ReceiveBeginPlay`
  (bind _asbp_player (cast `/Game/Blueprints/BP_Player` (`self.K2_GetPawn`)))
  (set `self.BP Player` _asbp_player))

(event `/Game/Blueprints/BP_TurnBasedObject.TickTurn`
  (`self.EnableInput` self))

(event `InputAction|MoveForward`
  (params (Key :type "Key Structure"))
  (:`Pressed`
    (`RogueLikePawn.MoveForward` (`self.BP Player`))))

(event `InputAction|MoveBackward`
  (params (Key :type "Key Structure"))
  (:`Pressed`
    (`RogueLikePawn.MoveBackward` (`self.BP Player`))))

(event `InputAction|MoveLeft`
  (params (Key :type "Key Structure"))
  (:`Pressed`
    (`RogueLikePawn.MoveLeft` (`self.BP Player`))))

(event `InputAction|MoveRight`
  (params (Key :type "Key Structure"))
  (:`Pressed`
    (`RogueLikePawn.MoveRight` (`self.BP Player`))))

(fn `UserConstructionScript`)