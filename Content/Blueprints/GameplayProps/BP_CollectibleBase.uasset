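; Base collectible prop Blueprint that handles the feedback and cleanup when the item is collected.
; Its Collect event plays a 2D pickup sound, activates the CollectVFX component and sets the mesh to ignore all collision channels, then destroys the actor after a short delay.
; IsCollected always returns false here, and a SpawnSystemAttached node is left unconnected.
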(event `/Game/Blueprints/BPI_Collectable.Collect`
  (`GameplayStatics.PlaySound2D` (`self.PickupSound`) 1.0 1.0 0.0 null null)
  (`ActorComponent.Activate` (`self.CollectVFX`) false)
  (`PrimitiveComponent.SetCollisionResponseToAllChannels` (`self.StaticMesh`) "ECR_Ignore")
  (`KismetSystemLibrary.Delay` 0.7)
  (`self.K2_DestroyActor`))

(fn `IsCollected`
  (returns (Result :type Boolean))
  (return false))

(fn `UserConstructionScript`)