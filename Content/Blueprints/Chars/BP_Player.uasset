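; BP_Player is a player Blueprint that can show either a static mesh or a skeletal mesh.
; SwapMesh takes a Static flag and sets opposite visibility on the two mesh components, without propagating to their children.
; It prints the active mesh type as debug text.
; The construction script is empty, and nothing in the file calls SwapMesh.
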(fn `SwapMesh`
  (params (Static :type Boolean))
  (if Static
    (`SceneComponent.SetVisibility` (`self.SkeletalMesh`) false false)
    (`SceneComponent.SetVisibility` (`self.StaticMesh`) true false)
    (`KismetSystemLibrary.PrintString` "Static")
    (else
      (`SceneComponent.SetVisibility` (`self.SkeletalMesh`) true false)
      (`SceneComponent.SetVisibility` (`self.StaticMesh`) false false)
      (`KismetSystemLibrary.PrintString` "Skeletal"))))

(fn `UserConstructionScript`)