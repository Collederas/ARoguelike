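; BP_Enemy is an enemy character Blueprint that gives visual and audio feedback when entering or leaving an alert state.
; At BeginPlay it caches and hides the WBP_Alert widget from its AlertSymbol component.
; EnterAlertMode plays the widget's appear animation and an alert sound while brightening the spotlight to red, then hides the widget when the animation finishes.
; ExitAlertMode restores a dimmer white light and plays a deactivation sound.
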(event `self.ReceiveBeginPlay`
  (bind _aswbp_alert (cast `/Game/UI/WBP_Alert` (`WidgetComponent.GetWidget` (`self.AlertSymbol`))))
  (bind _output_get (set `self.WBP Alert` _aswbp_alert))
  (`Widget.SetVisibility` _output_get "Collapsed"))

(event `/Game/Blueprints/BPI_Alertable.EnterAlertMode`
  (bind _wbp_alert (`self.WBP Alert`))
  (bind _spotlight (`self.SpotLight`))
  (bind _appearanimation (`/Game/UI/WBP_Alert.AppearAnimation` _wbp_alert))
  (`Widget.SetVisibility` _wbp_alert "Visible")
  (`UserWidget.BindToAnimationFinished` _wbp_alert _appearanimation (delegate `OnAlertAnimFinished`))
  (`UserWidget.PlayAnimation` _wbp_alert _appearanimation 0.0 1 "Forward" 1.0 false)
  (`GameplayStatics.PlaySoundAtLocation` "/Game/Audio/enemy_alert.enemy_alert" (`SceneComponent.K2_GetComponentLocation` (`self.AlertSymbol`)) (struct) 1.0 1.0 0.0 null null null)
  (`LightComponent.SetIntensity` _spotlight 10000.0)
  (`LightComponent.SetLightColor` _spotlight (struct :`R` 0.598958 :`G` 0.106002 :`B` 0.060264 :`A` 1.0) true))

(event `OnAlertAnimFinished`
  (`Widget.SetVisibility` (`self.WBP Alert`) "Collapsed"))

(event `/Game/Blueprints/BPI_Alertable.ExitAlertMode`
  (bind _spotlight (`self.SpotLight`))
  (`LightComponent.SetIntensity` _spotlight 3000.0)
  (`LightComponent.SetLightColor` _spotlight (struct :`R` 1.0 :`G` 1.0 :`B` 1.0 :`A` 1.0) true)
  (`GameplayStatics.PlaySoundAtLocation` "/Game/Audio/deactivate.deactivate" (`self.K2_GetActorLocation`) (struct) 1.0 1.0 0.0 null null null))

(fn `UserConstructionScript`)