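; Player controller for a turn-based, grid roguelike: handles movement input, potions, pause menu and switching between third-person and top-down cameras.
; Move starts a one-cell pawn move, then LocationCheck queries the WorldGrid to resolve walls, enemies, chests, potions or the goal.
; CanMove locks input during moves; successful completion spends a move and notifies listeners.
; TickTurn refills the move budget, and drinking a potion adds one.
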(event `self.ReceiveBeginPlay`
  (bind _returnvalue (`GameplayStatics.GetActorOfClass` "/Script/Roguelike.Grid"))
  (`/Engine/EditorBlueprintResources/StandardMacros.IsValid` _returnvalue
    (:`Is Valid`
      (set `self.WorldGrid` _returnvalue)
      (bind _returnvalue_2 (`|CreateWidget` "/Game/UI/WBP_HUD.WBP_HUD_C"))
      (bind _output_get (set `self.HUD` _returnvalue_2))
      (`UserWidget.AddToViewport` _output_get 0)
      (bind _returnvalue_3 (`|CreateWidget` "/Game/UI/WBP_PauseMenu.WBP_PauseMenu_C"))
      (set `self.PauseMenu` _returnvalue_3))
    (:`Is Not Valid`
      (`KismetSystemLibrary.PrintString` "Can't find WorldGrid in Level. Game can't continue" true true (struct :`R` 1.0 :`B` 0.039766 :`A` 1.0))
      (`KismetSystemLibrary.QuitGame` null "Quit"))))

(event `self.ReceivePossess`
  (params (PossessedPawn :type "Pawn Object Reference"))
  (`self.EnableInput` null)
  (bind _asbp_player (cast `/Game/Blueprints/Chars/BP_Player` PossessedPawn))
  (set `self.PlayerPawn` _asbp_player)
  (add `self.ReceiveMoveCompleted` (delegate `OnMoveCompleted`))
  (set `self.CanMove` true)
  (bind _asbp_roguelike_player_state (cast `/Game/Blueprints/BP_RoguelikePlayerState` (`self.PlayerState`)))
  (set `self.BP Roguelike Player State` _asbp_roguelike_player_state))

(event `OnMoveCompleted` :!signature `self.ReceiveMoveCompleted`
  (params (Result :type "EPathFollowingResult Enum" :default "Success"))
  (switch `EPathFollowingResult` Result
    (:`Success`
      (`/Engine/EditorBlueprintResources/StandardMacros.DecrementInt` (`self.AvailableMoves`)
        (:`  `
          (set `self.CanMove` true)
          (`self.NotifyMoveMade` self))))))

(event `/Game/Blueprints/BP_TurnBasedObject.TickTurn`
  (set `self.AvailableMoves` (`self.DefaultAvailableMoves`)))

(event `InputAction|MoveForward`
  (params (Key :type "Key Structure"))
  (:`Pressed`
    (`self.Move` "Forward")))

(event `InputAxis|TurnCamera`
  (params (AxisValue :type "Float (single-precision)"))
  ;[1 1 1] Camera
  (if (`|EnumEquality` "NewEnumerator0" (`self.CurrentCameraMode`))
    (`self.AddYawInput` AxisValue)))

(event `InputAction|Pause`
  (params (Key :type "Key Structure"))
  (bind _pausemenu (`self.PauseMenu`))
  (:`Pressed`
    (`/Engine/EditorBlueprintResources/StandardMacros.FlipFlop`
      (:`A`
        (`UserWidget.AddToViewport` _pausemenu 0)
        (`WidgetBlueprintLibrary.SetInputMode_UIOnlyEx` self _pausemenu)
        (set `self.bShowMouseCursor` true)
        (`self.DisableInput` self))
      (:`B`
        (`Widget.RemoveFromParent` _pausemenu)
        (`WidgetBlueprintLibrary.SetInputMode_GameOnly` self)
        (set `self.bShowMouseCursor` false)
        (`self.EnableInput` self)))))

(event `InputAction|MoveBackward`
  (params (Key :type "Key Structure"))
  (:`Pressed`
    (`self.Move` "Backward")))

(event `InputAxis|LookUp`
  (params (AxisValue :type "Float (single-precision)"))
  ;[1 1 1] Camera
  (if (`|EnumEquality` (`self.CurrentCameraMode`) "NewEnumerator0")
    (`self.AddPitchInput` (* AxisValue -1.0))))

(event `InputAction|MoveLeft`
  (params (Key :type "Key Structure"))
  (:`Pressed`
    (`self.Move` "Left")))

(event `InputAction|MoveRight`
  (params (Key :type "Key Structure"))
  (:`Pressed`
    (`self.Move` "Right")))

(event `InputAction|SwitchCamera`
  (params (Key :type "Key Structure"))
  (:`Pressed`
    (`/Engine/EditorBlueprintResources/StandardMacros.FlipFlop`
      (:`A`
        (`self.SetCameraMode` "NewEnumerator1"))
      (:`B`
        (`self.SetCameraMode` "NewEnumerator0")))))

(event `InputAction|UsePotion`
  (params (Key :type "Key Structure"))
  (:`Pressed`
    (if (and (> (`self.PotionsAmount`) 0) (`self.CanMove`))
      (`GameplayStatics.PlaySound2D` "/Game/Audio/Drink_Potion.Drink_Potion" 1.0 1.0 0.0 null null)
      (`NiagaraFunctionLibrary.SpawnSystemAtLocation` "/Game/Particles/NS_Burst.NS_Burst" (+ (`self.K2_GetActorLocation` (`self.K2_GetPawn`)) (0.0 0.0 30.0)))
      (`/Engine/EditorBlueprintResources/StandardMacros.IncrementInt` (`self.AvailableMoves`)
        (:`  `
          (`/Engine/EditorBlueprintResources/StandardMacros.DecrementInt` (`self.PotionsAmount`))))
      (else
        (`GameplayStatics.PlaySound2D` "/Game/Audio/denied.denied" 1.0 1.0 0.0 null null)))))

(fn `GetAvailableMoves`
  (returns (NrOfMovesLeft :type Integer))
  (return (`self.AvailableMoves`)))

(fn `LocationCheck`
  (params (Location :type "Vector Structure"))
  (bind _gridactor (`Grid.WorldPositionCheckGridOccupied` (`self.WorldGrid`) Location))
  (switch `EGridActorType` (`.ActorType` (break `GridActor` _gridactor))
    (:`Enemy`
      ;[1 0.02912 0.02604] Enemy
      (`self.MovingOnEnemy`)
      (`self.StopMovementImmediately`))
    (:`Wall`
      ;[0.1997 0.1997 0.1997] Wall
      (`GameplayStatics.PlaySound2D` "/Game/Audio/wall_thud.wall_thud" 1.0 1.0 0.0 null null)
      (`self.StopMovementImmediately`)
      (`KismetSystemLibrary.PrintString` "Can't move into walls, you silly")
      (set `self.CanMove` true))
    (:`Chest`
      ;[1 0.4218 0.1063] Chest
      (bind _result (message `/Game/Blueprints/BPI_Collectable.IsCollected` (break `GridActor` _gridactor)))
      (if _result
        (`GameplayStatics.PlaySound2D` "/Game/Audio/wall_thud.wall_thud" 1.0 1.0 0.0 null null)
        (`self.StopMovementImmediately`)
        (set `self.CanMove` true)
        (else
          (message `/Game/Blueprints/BPI_Collectable.Collect` (break `GridActor` _gridactor))
          (`self.StopMovementImmediately`)
          (`RoguelikePlayerState.AddKeys` (`self.BP Roguelike Player State`) 1)
          (set `self.CanMove` true))))
    (:`Potion`
      ;[0.02762 1 0.1224] Potion
      (`GameplayStatics.PlaySound2D` "/Game/Audio/footstep.footstep" 1.0 1.0 0.0 null null)
      (message `/Game/Blueprints/BPI_Collectable.Collect` (break `GridActor` _gridactor))
      (`/Engine/EditorBlueprintResources/StandardMacros.IncrementInt` (`self.PotionsAmount`)))
    (:`Goal`
      (message `/Game/Blueprints/BPI_Collectable.Collect` (break `GridActor` _gridactor))
      (`RoguelikePlayerState.IncrementLevel` (`self.BP Roguelike Player State`))
      (`self.LevelComplete`))
    (:`None`
      (`GameplayStatics.PlaySound2D` "/Game/Audio/footstep.footstep" 1.0 1.0 0.0 null null))))

(fn `Move`
  (params (Direction :type "EMoveDirection Enum" :default "Forward"))
  (locals (UpdatedLocation :type "Vector Structure" :default (0.0 0.0 0.0)))
  (bind _playerpawn (`self.PlayerPawn`))
  (if (`self.CanMove`)
    (set `self.CanMove` false)
    (switch `EMoveDirection` Direction
      (:`Forward`
        (bind _returnvalue (`RogueLikePawn.MoveForward` _playerpawn))
        (set `local.UpdatedLocation` _returnvalue))
      (:`Backward`
        (bind _returnvalue_2 (`RogueLikePawn.MoveBackward` _playerpawn))
        (set `local.UpdatedLocation` _returnvalue_2))
      (:`Left`
        (bind _returnvalue_3 (`RogueLikePawn.MoveLeft` _playerpawn))
        (set `local.UpdatedLocation` _returnvalue_3))
      (:`Right`
        (bind _returnvalue_4 (`RogueLikePawn.MoveRight` _playerpawn))
        (set `local.UpdatedLocation` _returnvalue_4)))
    (`self.LocationCheck` (`local.UpdatedLocation`))))

(fn `SetCameraMode`
  (params (RequestedMode :type "/Game/Blueprints/BP_ECameraModes Enum" :default "NewEnumerator0"))
  (locals (LookupActiveCameraTag :type Name) (LookupDisableCameraTag :type Name))
  (switch `/Game/Blueprints/BP_ECameraModes` RequestedMode
    (:`NewEnumerator0`
      (set `local.LookupActiveCameraTag` (`self.ThirdPersonCameraTag`))
      (set `local.LookupDisableCameraTag` (`self.TopDownCameraTag`))
      (set `self.CurrentCameraMode` "NewEnumerator0"))
    (:`NewEnumerator1`
      (set `local.LookupActiveCameraTag` (`self.TopDownCameraTag`))
      (set `local.LookupDisableCameraTag` (`self.ThirdPersonCameraTag`))
      (set `self.CurrentCameraMode` "NewEnumerator1")))
  (`ActorComponent.SetActive` (`|GetArrayItem` (`self.GetComponentsByTag` (`self.PlayerPawn`) "/Script/Engine.CameraComponent" (`local.LookupActiveCameraTag`))) true false)
  (`ActorComponent.SetActive` (`|GetArrayItem` (`self.GetComponentsByTag` (`self.PlayerPawn`) "/Script/Engine.CameraComponent" (`local.LookupDisableCameraTag`))) false false)
  (`self.SetControlRotation` (`KismetMathLibrary.MakeRotator` 0.0)))

(fn `StopMovementImmediately`
  (`MovementComponent.StopMovementImmediately` (`Pawn.GetMovementComponent` (`self.PlayerPawn`))))

(fn `UserConstructionScript`)