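; AI controller for a turn-based, grid-moving enemy that steps toward the player and tracks whether it has noticed them.
; Each turn it retargets its path-following component to the player, moves one grid step and plays a drag sound, regardless of alert state.
; Perception triggers alert mode through BPI_Alertable; completed moves count unseen turns toward exiting it.
; Successful moves report out of moves, and nearing the target fires a target-reached notification.
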(event `self.ReceivePossess`
  (params (PossessedPawn :type "Pawn Object Reference"))
  (bind _asbp_player_controller (cast `/Game/Blueprints/Chars/BP_PlayerController` (`GameplayStatics.GetPlayerController` 0)))
  (set `self.PlayerController` _asbp_player_controller))

(event `/Game/Blueprints/BP_TurnBasedObject.TickTurn`
  (`self.Move`))

(event `self.OnMoveCompleted_Blueprint`
  (params (RequestID :type "AIRequestID Structure") (Result :type "EPathFollowingResult Enum" :default "Success"))
  (switch `EPathFollowingResult` Result
    (:`Success`
      (if (`self.PlayerSensed`)
        _
        (elif (< (`self.PlayerSensedElapsedTurns`) (`self.ForgetPlayerAfterNTurns`))
          (`/Engine/EditorBlueprintResources/StandardMacros.IncrementInt` (`self.PlayerSensedElapsedTurns`)
            (:`  `
              _))
          (else
            (set `self.FollowingPlayer` false)
            (message `/Game/Blueprints/BPI_Alertable.ExitAlertMode` (`self.K2_GetPawn`)))))
      (`self.NotifyOutOfMoves` self))))

(event `self.OnAboutToReachTarget`
  (`self.TargetReached`))

(event `self.AIPerception.OnTargetPerceptionUpdated`
  (params (Actor :type "Actor Object Reference") (Stimulus :type "AIStimulus Structure"))
  (bind _returnvalue (`self.K2_GetPawn`))
  (if (and (`self.ActorHasTag` Actor "Player") Stimulus_bSuccessfullySensed)
    (set `self.PlayerSensed` true)
    (if (not (`self.FollowingPlayer`))
      (set `self.FollowingPlayer` true)
      (set `self.PlayerSensedElapsedTurns` 0)
      (if (`KismetSystemLibrary.DoesImplementInterface` _returnvalue "/Game/Blueprints/BPI_Alertable.BPI_Alertable_C")
        (message `/Game/Blueprints/BPI_Alertable.EnterAlertMode` _returnvalue)))
    (else
      (set `self.PlayerSensed` false))))

(fn `GetAvailableMoves`
  (returns (NrOfMovesLeft :type Integer))
  (return 0))

(fn `GridMoveToLocation`
  (params (Location :type "Vector Structure") (NumberOfMoves :type Integer))
  (`self.GridMoveTo` Location null NumberOfMoves))

(fn `Move`
  (bind _returnvalue (`self.K2_GetActorLocation` (`GameplayStatics.GetPlayerPawn` 0)))
  (bind _returnvalue_2 (`self.K2_GetActorLocation` (`self.K2_GetPawn`)))
  (bind _returnvalue_3 (`self.GetRLPathFollowingComponent`))
  (`RoguelikePathFollowingComponent.UpdateTargetLocation` _returnvalue_3 (`KismetMathLibrary.Conv_VectorToVector2D` _returnvalue))
  (set `self.LocationAtTurnStart` _returnvalue_2)
  (`self.GridMoveTo` _returnvalue null 1)
  (`GameplayStatics.PlaySoundAtLocation` "/Game/Audio/drag_1.drag_1" _returnvalue_2 (struct) 1.0 1.0 0.0 null null null))

(fn `UserConstructionScript`)