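; Game mode for a turn-based roguelike that runs level spawning, player and enemy turns, and game-over restarts.
; After BP_LevelSpawner builds a level, it collects enemy controllers and binds their events.
; A FlipFlop alternates turns, skipping the enemy turn when none are alerted and otherwise counting out-of-moves notifications until all alerted enemies finish.
; Player moving onto an enemy or enemies reaching their target triggers a delayed pawn destruction and restart.
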(event `RestartGame`
  (bind _returnvalue (`GameplayStatics.GetPlayerController` 0))
  (bind _levelspawner (`self.LevelSpawner`))
  (`self.RestartPlayer` _returnvalue)
  (bind _asbp_player_controller (cast `/Game/Blueprints/BP_PlayerController` _returnvalue))
  (set `self.PlayerController` _asbp_player_controller)
  (`LevelSpawner.SpawnNewLevel` _levelspawner :!label _label)
  (bind _controllers (`self.CollectEnemyControllers` _levelspawner))
  (for _ _controllers
    (add `/Game/Blueprints/BP_EnemyController.NotifyOutOfMoves` _controllers (delegate `OnObjectOutOfMoves`))
    (add `/Game/Blueprints/BP_EnemyController.TargetReached` _controllers (delegate `GameOver`)))
  (`self.TickTurn`))

(event `self.ReceiveBeginPlay`
  (bind _playercontroller (`self.PlayerController`))
  (bind _asbp_player_controller (cast `/Game/Blueprints/BP_PlayerController` (`GameplayStatics.GetPlayerController` 0)))
  (set `self.PlayerController` _asbp_player_controller)
  (bind _returnvalue (`GameplayStatics.GetActorOfClass` "/Game/Blueprints/BP_LevelSpawner.BP_LevelSpawner_C"))
  (set `self.LevelSpawner` _returnvalue)
  (add `/Game/Blueprints/BP_PlayerController.NotifyMoveMade` _playercontroller (delegate `OnObjectOutOfMoves`))
  (add `/Game/Blueprints/BP_PlayerController.MovingOnEnemy` _playercontroller (delegate `GameOver`))
  (goto _label))

(event `GameOver`
  (`KismetSystemLibrary.Delay` 1.2)
  (`self.K2_DestroyActor` (`Controller.K2_GetPawn` (`self.PlayerController`)))
  (`self.RestartGame`))

(event `self.TickTurn`
  (`/Engine/EditorBlueprintResources/StandardMacros.FlipFlop`
    (:`A`
      (set `self.TurnOwner` "NewEnumerator0")
      (`KismetSystemLibrary.PrintString` "Player's Turn")
      (`self.TickTurn` (`self.PlayerController`)))
    (:`B`
      (set `self.TurnOwner` "NewEnumerator1")
      (set `self.NrOfEnemiesOutOfMoves` 0)
      (bind (_alertedenemies _isempty) (`self.GetAlertedEnemies`))
      (if _isempty
        (`self.TickTurn`)
        (else
          (`KismetSystemLibrary.PrintString` "Enemies Turn" true true (struct :`R` 1.0 :`G` 0.889804 :`B` 0.136031 :`A` 1.0))
          (set `self.AlertedEnemies` _alertedenemies)
          (`self.TickTurn` _alertedenemies))))))

(event `OnObjectOutOfMoves`
  (params (TurnBasedObject :type "/Game/Blueprints/BP_TurnBasedObject Interface"))
  (switch `/Game/Blueprints/BP_EFactions` (`self.TurnOwner`)
    (:`NewEnumerator0`
      (`self.TickTurn`))
    (:`NewEnumerator1`
      (bind _result (`/Engine/EditorBlueprintResources/StandardMacros.IncrementInt` (`self.NrOfEnemiesOutOfMoves`))
        (:`  `
          (if (== _result (`KismetArrayLibrary.Array_Length` (`self.AlertedEnemies`)))
            (`self.TickTurn`)))))))

(fn `CollectEnemyControllers`
  (params (LevelSpawner :type "LevelSpawner Object Reference"))
  (returns (Controllers :type "Array of /Game/Blueprints/BP_EnemyController Object Reference"))
  (`KismetArrayLibrary.Array_Clear` (`self.EnemyControllers`))
  (bind _returnvalue (`LevelSpawner.GetAllEnemies` LevelSpawner))
  (for _array_element _returnvalue
    (bind _asbp_enemy_controller (cast `/Game/Blueprints/BP_EnemyController` (`AIBlueprintHelperLibrary.GetAIController` _array_element)))
    (`KismetArrayLibrary.Array_AddUnique` (`self.EnemyControllers`) _asbp_enemy_controller))
  (return (`self.EnemyControllers`)))

(fn `GetAlertedEnemies`
  (returns (AlertedEnemies :type "Array of /Game/Blueprints/BP_EnemyController Object Reference") (IsEmpty :type Boolean))
  (locals (Result :type "Array of /Game/Blueprints/BP_EnemyController Object Reference"))
  (bind _result (`local.Result`))
  (for _array_element (`self.EnemyControllers`)
    (if (`/Game/Blueprints/BP_EnemyController.Alerted` _array_element)
      (`KismetArrayLibrary.Array_AddUnique` (`local.Result`) _array_element)))
  (return _result (`KismetArrayLibrary.Array_IsEmpty` _result)))

(fn `GetAvailableMoves`
  (returns (NrOfMovesLeft :type Integer))
  (return 0))

(fn `UserConstructionScript`)